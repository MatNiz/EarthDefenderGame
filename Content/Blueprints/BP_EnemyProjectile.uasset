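; BP_EnemyProjectile is an enemy projectile actor that reacts when its static mesh overlaps the player or the Earth.
; On overlap it compares the other actor's exact class against BP_MyPlayer and BP_Earth.
; A player hit destroys the projectile and calls GetHit on BP_GameMode, so the game mode handles the hit.
; An Earth hit only destroys the projectile, and the graph contains no movement logic.
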(event `self.StaticMeshComponent.OnComponentBeginOverlap`
  (params (OverlappedComponent :type "PrimitiveComponent Object Reference") (OtherActor :type "Actor Object Reference") (OtherComp :type "PrimitiveComponent Object Reference") (OtherBodyIndex :type Integer) (bFromSweep :type Boolean) (SweepResult :type "HitResult Structure (by ref)"))
  (bind _returnvalue (`GameplayStatics.GetObjectClass` OtherActor))
  (`|ExecutionSequence`
    (:`then_0`
      (if (== _returnvalue "/Game/Blueprints/BP_MyPlayer.BP_MyPlayer_C")
        (`self.K2_DestroyActor`)
        (bind _asbp_game_mode (cast `/Game/Blueprints/BP_GameMode` (`GameplayStatics.GetGameMode`)))
        (`/Game/Blueprints/BP_GameMode.GetHit` _asbp_game_mode true)))
    (:`then_1`
      (if (== _returnvalue "/Game/Blueprints/BP_Earth.BP_Earth_C")
        (`self.K2_DestroyActor`)))))

(fn `UserConstructionScript`)