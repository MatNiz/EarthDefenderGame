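; Game mode for an asteroid shooter that tracks player HP, live threat counts and the win or loss end state.
; BeginPlay sets HP and shows the UI widget, while Tick recounts asteroids and enemies every frame through GetAllActorsOfClass.
; GetHit decrements HP and calls GameEnd at zero, which shows the end screen, switches to UI-only input and destroys spawners, asteroids and enemies.
; CheckIfWin returns true once no enemies or asteroids remain.
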(event `self.ReceiveBeginPlay`
  (set `self.HP` 3)
  (bind _returnvalue (`|CreateWidget` "/Game/Blueprints/WBP_UI.WBP_UI_C"))
  (`UserWidget.AddToViewport` _returnvalue 0))

(event `self.ReceiveTick`
  (params (DeltaSeconds :type "Float (single-precision)"))
  (bind _outactors (`GameplayStatics.GetAllActorsOfClass` "/Game/Blueprints/BP_Asteroid.BP_Asteroid_C"))
  (set `self.NumberOfAsteroids` (`KismetArrayLibrary.Array_Length` _outactors))
  (bind _outactors_2 (`GameplayStatics.GetAllActorsOfClass` "/Game/Blueprints/BP_Enemy.BP_Enemy_C"))
  (set `self.NumberOfEnemies` (`KismetArrayLibrary.Array_Length` _outactors_2)))

(fn `CheckIfWin`
  (returns (Win :type Boolean))
  (bind _outactors (`GameplayStatics.GetAllActorsOfClass` "/Game/Blueprints/BP_Enemy.BP_Enemy_C"))
  (if (== (`KismetArrayLibrary.Array_Length` _outactors) 0)
    (bind _outactors_2 (`GameplayStatics.GetAllActorsOfClass` "/Game/Blueprints/BP_Asteroid.BP_Asteroid_C"))
    (if (`KismetArrayLibrary.Array_IsEmpty` _outactors_2)
      (return true)
      (else
        _)))
  (return false))

(fn `Game End`
  (params (LostGame :type Boolean))
  (bind _returnvalue (`GameplayStatics.GetPlayerController` 0))
  (bind _returnvalue_2 (`|CreateWidget` "/Game/Blueprints/WBP_EndScreen.WBP_EndScreen_C" null LostGame))
  (`UserWidget.AddToViewport` _returnvalue_2 0)
  (`WidgetBlueprintLibrary.SetInputMode_UIOnlyEx` _returnvalue _returnvalue_2)
  (`Controller.SetIgnoreMoveInput` _returnvalue false)
  (`|ExecutionSequence`
    (:`then_0`
      (bind _outactors (`GameplayStatics.GetAllActorsOfClass` "/Game/Blueprints/BP_AsteroidSpawner.BP_AsteroidSpawner_C"))
      (for _array_element _outactors
        (`self.K2_DestroyActor` _array_element)))
    (:`then_1`
      (bind _outactors_2 (`GameplayStatics.GetAllActorsOfClass` "/Game/Blueprints/BP_Asteroid.BP_Asteroid_C"))
      (for _array_element_2 _outactors_2
        (`self.K2_DestroyActor` _array_element_2)))
    (:`then_2`
      (bind _outactors_3 (`GameplayStatics.GetAllActorsOfClass` "/Game/Blueprints/BP_Enemy.BP_Enemy_C"))
      (for _array_element_3 _outactors_3
        (`self.K2_DestroyActor` _array_element_3)))))

(fn `GetHit`
  (params (LostGame :type Boolean))
  (bind _result (`/Engine/EditorBlueprintResources/StandardMacros.DecrementInt` (`self.HP`))
    (:`  `
      (bind _output_get (set `self.HP` _result))
      (if (== _output_get 0)
        (`self.Game End` LostGame)))))

(fn `UserConstructionScript`)