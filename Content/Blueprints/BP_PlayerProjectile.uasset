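; BP_PlayerProjectile is the player's projectile, which resolves hits when its static mesh begins overlapping another actor.
; It destroys itself on enemies, special enemies, asteroids and Earth, destroying either enemy type and calling Decay on asteroids.
; Enemy and asteroid hits then ask BP_GameMode to check for a win and end the game, while special-enemy hits skip that check.
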(event `self.StaticMeshComponent.OnComponentBeginOverlap`
  (params (OverlappedComponent :type "PrimitiveComponent Object Reference") (OtherActor :type "Actor Object Reference") (OtherComp :type "PrimitiveComponent Object Reference") (OtherBodyIndex :type Integer) (bFromSweep :type Boolean) (SweepResult :type "HitResult Structure (by ref)"))
  (bind _returnvalue (`GameplayStatics.GetObjectClass` OtherActor))
  (`|ExecutionSequence`
    (:`then_0`
      (if (== _returnvalue "/Game/Blueprints/BP_Enemy.BP_Enemy_C")
        (`self.K2_DestroyActor`)
        (`self.K2_DestroyActor` OtherActor)
        (bind _asbp_game_mode (cast `/Game/Blueprints/BP_GameMode` (`GameplayStatics.GetGameMode`) :!label _label))
        (bind _win (`/Game/Blueprints/BP_GameMode.CheckIfWin` _asbp_game_mode))
        (if _win
          (`/Game/Blueprints/BP_GameMode.Game End` _asbp_game_mode false))))
    (:`then_1`
      (bind _outactors (`GameplayStatics.GetAllActorsOfClass` "/Game/Blueprints/BP_Asteroid.BP_Asteroid_C"))
      (for _array_element _outactors
        (if (== _array_element OtherActor)
          (`self.K2_DestroyActor`)
          (`Asteroid.Decay` _array_element)
          (goto _label))))
    (:`then_2`
      (if (== _returnvalue "/Game/Blueprints/BP_Earth.BP_Earth_C")
        (`self.K2_DestroyActor`)))
    (:`then_3`
      (if (== (`GameplayStatics.GetObjectClass` OtherActor) "/Game/Blueprints/BP_EnemySpecial.BP_EnemySpecial_C")
        (`self.K2_DestroyActor`)
        (`self.K2_DestroyActor` OtherActor)))))

(fn `UserConstructionScript`)